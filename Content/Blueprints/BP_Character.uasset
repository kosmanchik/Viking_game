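; Character Blueprint for sword melee combat with an endurance-limited combo attack and damage intake.
; Left click spends endurance, calls RestoreEndurance, and either plays the combo montage or queues the next hit.
; Montage notifies consume the queued input and blend out the montage when none remains.
; TrigeredAttack and StopSword toggle a fast looping timer tracing between sword sockets, while AnyDamage feeds UpdateHealth.
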(event Custom|TrigeredAttack
  (bind _returnvalue (Utilities|Time|SetTimerbyEvent (delegate Custom|SwordLinetrace) 0.01 true))
  (Variables|Default|SetTimerSwordEvent _returnvalue))

(event Custom|SwordLinetrace
  (bind _mesh (Variables|Character|GetMesh))
  (Class|CPPCharacter|SwordTrace (Transformation|GetSocketLocation _mesh "start") (Transformation|GetSocketLocation _mesh "end")))

(event Custom|StopSword
  (Utilities|Time|ClearandInvalidateTimerbyHandle (Variables|Default|GetTimerSwordEvent)))

(event EventTick
  (params (DeltaSeconds :type Float%20%28single-precision%29)))

(event Game|Damage|EventAnyDamage
  (params (Damage :type Float%20%28single-precision%29) (DamageType :type Damage%20Type%20Object%20Reference) (InstigatedBy :type Controller%20Object%20Reference) (DamageCauser :type Actor%20Object%20Reference))
  (Class|CPPCharacter|UpdateHealth Damage))

(event Input|MouseEvents|LeftMouseButton
  (params (Key :type Key%20Structure :default "None"))
  (:Pressed
    (if (> (Variables|Default|GetEndurance) 0.0)
      (if (Animation|Montage|MontageIsPlaying (Components|SkeletalMesh|GetAnimInstance (Variables|Character|GetMesh)) "/Game/Characters/Others/Anim/MainAnim/AM_ComboAttack.AM_ComboAttack")
        (Variables|Default|Setattackindex 1)
        (Variables|Default|SetEndurance (- (Variables|Default|GetEndurance) 15.0))
        (Class|CPPCharacter|RestoreEndurance)
        (else
          (Variables|Default|SetEndurance (- (Variables|Default|GetEndurance) 15.0))
          (Class|CPPCharacter|RestoreEndurance)
          (Animation|Montage|PlayMontage (Variables|Character|GetMesh) "/Game/Characters/Others/Anim/MainAnim/AM_ComboAttack.AM_ComboAttack"
            (:OnNotifyBegin
              (bind _result (Math|Integer|DecrementInt (Variables|Default|Getattackindex))
                (:%20%20
                  (if (< _result 0)
                    (Animation|Montage|MontageStop (Components|SkeletalMesh|GetAnimInstance (Variables|Character|GetMesh)) 0.35 "/Game/Characters/Others/Anim/MainAnim/AM_ComboAttack.AM_ComboAttack")
                    (Variables|Default|Setattackindex 0)))))))))))

(fn ConstructionScript)