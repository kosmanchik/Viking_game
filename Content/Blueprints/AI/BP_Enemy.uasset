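; BP_Enemy is an AI enemy pawn that spots the player, attacks with a sword and takes damage.
; PawnSensing sets the HasSeenPlayer blackboard key when it sees BP_Character, and incoming damage feeds UpdateHealth.
; AttackPlayer sphere-traces for the player, plays a slash montage, waits its length, then line-traces along the sword sockets.
; Damage goes to the sphere-traced character regardless of the sword trace result.
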(event OnSeePawn(PawnSensing)
  (params (Pawn :type Pawn%20Object%20Reference))
  (Utilities|Casting|CastToBP_Character Pawn)
  (AI|Components|Blackboard|SetValueasBool (AI|GetBlackboard (AI|GetAIController self)) (Utilities|Name|MakeLiteralName "HasSeenPlayer") true))

(event Custom|AttackPlayer
  (bind _sword (Variables|Default|GetSword))
  (bind _returnvalue (Class|CPPEnemy|SphereTracebyChase))
  (bind _asbp_character (Utilities|Casting|CastToBP_Character (.HitActor (Collision|BreakHitResult _returnvalue))))
  (bind _returnvalue_2 (Animation|PlayAnimMontage "/Game/FightSystem/Slash_Montage.Slash_Montage" 1.0 "None"))
  (Utilities|FlowControl|Delay _returnvalue_2)
  (Class|CPPEnemy|LineTracebySword (Transformation|GetSocketLocation _sword "Start") (Transformation|GetSocketLocation _sword "End"))
  (Game|Damage|ApplyDamage _asbp_character 5.0 0 0))

(event EventBeginPlay)

(event Collision|EventActorBeginOverlap
  (params (OtherActor :type Actor%20Object%20Reference)))

(event EventTick
  (params (DeltaSeconds :type Float%20%28single-precision%29)))

(event Game|Damage|EventAnyDamage
  (params (Damage :type Float%20%28single-precision%29) (DamageType :type Damage%20Type%20Object%20Reference) (InstigatedBy :type Controller%20Object%20Reference) (DamageCauser :type Actor%20Object%20Reference))
  (Class|CPPEnemy|UpdateHealth Damage))

(fn ConstructionScript)